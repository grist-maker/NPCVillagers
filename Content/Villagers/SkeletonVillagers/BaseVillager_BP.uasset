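; Base Blueprint for villager NPCs that handles conversation, hit and gift reactions, and animation state.
; Every tick it copies its State into the cached NPCController_ABP anim instance.
; Talk branches on a topic string to pick a line from its DialogBank component, while Hit and Gift fetch reaction lines from the same bank.
; Responses are written to the DialogBox widget held by the player's PlayerVillager_BP pawn.
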(event `self.ReceiveBeginPlay`
  (bind _asnpccontroller_abp (cast `/Game/AnimationControllers/NPCController_ABP` (`SkeletalMeshComponent.GetAnimInstance` (`self.Mesh`))))
  (set `self.AnimationBlueprint` _asnpccontroller_abp))

(event `self.ReceiveTick`
  (params (DeltaSeconds :type "Float (single-precision)"))
  (set `/Game/AnimationControllers/NPCController_ABP.CurrentState` (`self.State`) (`self.AnimationBlueprint`)))

(event `Talk`
  (params (Topic :type String))
  (bind _returnvalue (`self.GetComponentByClass` "/Script/NPCVillagers.DialogBank"))
  (if (`KismetStringLibrary.EqualEqual_StrStr` Topic "Job")
    (bind _returnvalue_2 (`DialogBank.SelectWorkResponse` _returnvalue))
    (`self.Print To Screen` _returnvalue_2)
    (elif (`KismetStringLibrary.EqualEqual_StrStr` Topic "Mood")
      (bind _returnvalue_3 (`DialogBank.SelectMoodResponse` _returnvalue))
      (`self.Print To Screen` _returnvalue_3)
      (elif (`KismetStringLibrary.EqualEqual_StrStr` Topic "Energy")
        (bind _returnvalue_4 (`DialogBank.SelectEnergyResponse` _returnvalue))
        (`self.Print To Screen` _returnvalue_4)
        (elif (`KismetStringLibrary.EqualEqual_StrStr` Topic "Relationship")
          (bind _returnvalue_5 (`DialogBank.SelectRelationshipResponse` _returnvalue))
          (`self.Print To Screen` _returnvalue_5)
          (elif (`KismetStringLibrary.EqualEqual_StrStr` Topic "Anything")
            (bind _returnvalue_6 (`DialogBank.SelectRandomResponse` _returnvalue))
            (`self.Print To Screen` _returnvalue_6)
            (elif (`KismetStringLibrary.EqualEqual_StrStr` Topic "Generic")
              (bind _returnvalue_7 (`DialogBank.SelectGenericResponse` _returnvalue))
              (`self.Print To Screen` _returnvalue_7)
              (elif (`KismetStringLibrary.EqualEqual_StrStr` Topic "Coworker")
                (bind _returnvalue_8 (`DialogBank.SelectCoworkerResponse` _returnvalue))
                (`self.Print To Screen` _returnvalue_8)))))))))

(event `Print To Screen`
  (params (Message :type String))
  (set `TextBlock.Text` (`KismetTextLibrary.Conv_StringToText` Message) (`/Game/UI/DialogBox.InnerText` (cast `/Game/UI/DialogBox` (`/Game/Player/PlayerVillager_BP.Textbox` (cast `/Game/Player/PlayerVillager_BP` (`GameplayStatics.GetPlayerPawn` 0) :!pure true)) :!pure true))))

(event `Hit`
  (bind _returnvalue (`DialogBank.HurtReaction` (`self.GetComponentByClass` "/Script/NPCVillagers.DialogBank")))
  (`self.Print To Screen` _returnvalue))

(event `Gift`
  (params (Name :type String))
  (bind _returnvalue (`DialogBank.GiftReaction` (`self.GetComponentByClass` "/Script/NPCVillagers.DialogBank") Name))
  (set `TextBlock.Text` (`KismetTextLibrary.Conv_StringToText` _returnvalue) (`/Game/UI/DialogBox.InnerText` (cast `/Game/UI/DialogBox` (`/Game/Player/PlayerVillager_BP.Textbox` (cast `/Game/Player/PlayerVillager_BP` (`GameplayStatics.GetPlayerPawn` 0) :!pure true)) :!pure true))))

(fn `UserConstructionScript`)