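; Shy villager personality Blueprint that shows the villager's stats on an NPCStats widget held by its Stats component.
; BeginPlay calls the parent and writes the name label once.
; Tick calls the parent, then rewrites affinity, energy, mood and emotion labels every frame by casting the widget and setting text directly.
; No shy-specific logic appears in these graphs, and the construction script only calls the parent.
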(event `self.ReceiveBeginPlay`
  (`parent.ReceiveBeginPlay`)
  (set `TextBlock.Text` (`KismetTextLibrary.Conv_StringToText` (`KismetStringLibrary.Concat_StrStr` (`KismetTextLibrary.Conv_TextToString` (`|FormatText` "Name: ")) (`self.Name`))) (`/Game/UI/NPCStats.Name` (cast `/Game/UI/NPCStats` (`WidgetComponent.GetWidget` (`self.Stats`)) :!pure true))))

(event `self.ReceiveTick`
  (params (DeltaSeconds :type "Float (single-precision)"))
  (bind _asnpcstats (cast `/Game/UI/NPCStats` (`WidgetComponent.GetWidget` (`self.Stats`)) :!pure true))
  (`parent.ReceiveTick` DeltaSeconds)
  (set `TextBlock.Text` (`KismetTextLibrary.Conv_StringToText` (`KismetStringLibrary.Concat_StrStr` (`KismetTextLibrary.Conv_TextToString` (`|FormatText` "Affinity: ")) (`KismetStringLibrary.Conv_DoubleToString` (`self.PlayerAffinity`)))) (`/Game/UI/NPCStats.Affinity` _asnpcstats))
  (set `TextBlock.Text` (`KismetTextLibrary.Conv_StringToText` (`KismetStringLibrary.Concat_StrStr` (`KismetTextLibrary.Conv_TextToString` (`|FormatText` "Energy:")) (`KismetStringLibrary.Conv_DoubleToString` (`self.Energy`)))) (`/Game/UI/NPCStats.Energy` _asnpcstats))
  (set `TextBlock.Text` (`KismetTextLibrary.Conv_StringToText` (`KismetStringLibrary.Concat_StrStr` (`KismetTextLibrary.Conv_TextToString` (`|FormatText` "Mood:")) (`|GetEnumeratorNameAsString` (`self.Mood`)))) (`/Game/UI/NPCStats.Mood` _asnpcstats))
  (set `TextBlock.Text` (`KismetTextLibrary.Conv_StringToText` (`KismetStringLibrary.Concat_StrStr` (`KismetTextLibrary.Conv_TextToString` (`|FormatText` "Happiness:")) (`KismetStringLibrary.Conv_DoubleToString` (`self.Happiness`)))) (`/Game/UI/NPCStats.Happiness` _asnpcstats))
  (set `TextBlock.Text` (`KismetTextLibrary.Conv_StringToText` (`KismetStringLibrary.Concat_StrStr` (`KismetTextLibrary.Conv_TextToString` (`|FormatText` "Sadness:")) (`KismetStringLibrary.Conv_DoubleToString` (`self.Sadness`)))) (`/Game/UI/NPCStats.Sadness` _asnpcstats))
  (set `TextBlock.Text` (`KismetTextLibrary.Conv_StringToText` (`KismetStringLibrary.Concat_StrStr` (`KismetTextLibrary.Conv_TextToString` (`|FormatText` "Excitement:")) (`KismetStringLibrary.Conv_DoubleToString` (`self.Excitement`)))) (`/Game/UI/NPCStats.Excitement` _asnpcstats))
  (set `TextBlock.Text` (`KismetTextLibrary.Conv_StringToText` (`KismetStringLibrary.Concat_StrStr` (`KismetTextLibrary.Conv_TextToString` (`|FormatText` "Anger:")) (`KismetStringLibrary.Conv_DoubleToString` (`self.Anger`)))) (`/Game/UI/NPCStats.Anger` _asnpcstats))
  (set `TextBlock.Text` (`KismetTextLibrary.Conv_StringToText` (`KismetStringLibrary.Concat_StrStr` (`KismetTextLibrary.Conv_TextToString` (`|FormatText` "Fear:")) (`KismetStringLibrary.Conv_DoubleToString` (`self.Fear`)))) (`/Game/UI/NPCStats.Fear` _asnpcstats)))

(fn `UserConstructionScript`
  (`parent.UserConstructionScript`))