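; Player villager Blueprint that lets the player hit, gift or talk to NPC villagers and shows the in-game day and time.
; BeginPlay creates the HUD, dialog and menu widgets, and Tick refreshes the clock from TimeManager_BP.
; Interact traces forward for a BaseVillager_BP and opens a UI-only menu, or ends an active dialog.
; Choice events forward the action, gift name or topic to that NPC, show the textbox and restore game input.
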(event `self.ReceiveBeginPlay`
  (bind _returnvalue (`GameplayStatics.GetActorOfClass` "/Game/Managers/TimeManager_BP.TimeManager_BP_C"))
  (set `self.Manager` _returnvalue)
  (bind _returnvalue_2 (`|CreateWidget` "/Game/UI/DateTimeDisplay.DateTimeDisplay_C"))
  (`UserWidget.AddToViewport` _returnvalue_2 0)
  (bind _returnvalue_3 (`|CreateWidget` "/Game/UI/DialogBox.DialogBox_C"))
  (bind _output_get (set `self.Textbox` _returnvalue_3))
  (`UserWidget.AddToViewport` _output_get 0)
  (`Widget.SetVisibility` _output_get "Hidden")
  (bind _returnvalue_4 (`|CreateWidget` "/Game/UI/InteractMenu.InteractMenu_C"))
  (bind _output_get_2 (set `self.InteractMenu` _returnvalue_4))
  (`UserWidget.AddToViewport` _output_get_2 0)
  (`Widget.SetVisibility` _output_get_2 "Collapsed")
  (bind _returnvalue_5 (`|CreateWidget` "/Game/UI/GiftUI.GiftUI_C"))
  (bind _output_get_3 (set `self.GiftName` _returnvalue_5))
  (`UserWidget.AddToViewport` _output_get_3 0)
  (`Widget.SetVisibility` _output_get_3 "Collapsed")
  (bind _returnvalue_6 (`|CreateWidget` "/Game/UI/TalkMenu.TalkMenu_C"))
  (bind _output_get_4 (set `self.DialogMenu` _returnvalue_6))
  (`UserWidget.AddToViewport` _output_get_4 0)
  (`Widget.SetVisibility` _output_get_4 "Collapsed"))

(event `InputAction|Interact`
  (params (Key :type "Key Structure"))
  (bind _returnvalue (`self.K2_GetActorLocation`))
  (:`Pressed`
    (if (`self.Interacting`)
      (`self.CleanUI`)
      (set `self.Interacting` false)
      (`BaseVillager.EndDialog` (`self.InteractedNPC`))
      (else
        (bind _outhit (`KismetSystemLibrary.LineTraceSingleForObjects` _returnvalue (+ _returnvalue (* (`self.GetActorForwardVector`) (500.0 500.0 500.0))) (`|MakeArray` (enumliteral `EObjectTypeQuery` "ObjectTypeQuery3"))))
        (bind _asbase_villager_bp (cast `/Game/Villagers/SkeletonVillagers/BaseVillager_BP` (`.HitActor` (`GameplayStatics.BreakHitResult` _outhit))))
        (set `self.InteractedNPC` _asbase_villager_bp)
        (`self.OpenInteract`)))))

(event `self.ReceiveTick`
  (params (DeltaSeconds :type "Float (single-precision)"))
  (bind (_currenttime_hour _currenttime_minute) (break `Timestamp` (`TimeManager.CurrentTime` (`self.Manager`))))
  (bind (_currenttime_hour_2 _currenttime_minute_2) (break `Timestamp` (`TimeManager.CurrentTime` (`self.Manager`))))
  (`TextBlock.SetText` (`/Game/UI/DateTimeDisplay.Day` (stale `self.ReceiveBeginPlay` _returnvalue_2)) (`KismetTextLibrary.Conv_StringToText` (`KismetStringLibrary.Concat_StrStr` (`KismetTextLibrary.Conv_TextToString` (`|FormatText` "Day: ")) (`|GetEnumeratorNameAsString` (`TimeManager.CurrentDay` (`self.Manager`))))))
  (if (< _currenttime_minute 10)
    (bind _time (`/Game/UI/DateTimeDisplay.Time` (stale `self.ReceiveBeginPlay` _returnvalue_2)))
    (`TextBlock.SetText` _time (`KismetTextLibrary.Conv_StringToText` (`KismetStringLibrary.Concat_StrStr` (`KismetTextLibrary.Conv_TextToString` (`|FormatText` "Time: ")) (`KismetStringLibrary.Conv_IntToString` _currenttime_hour_2) ":" "0" (`KismetStringLibrary.Conv_IntToString` _currenttime_minute_2))))
    (else
      (`TextBlock.SetText` _time (`KismetTextLibrary.Conv_StringToText` (`KismetStringLibrary.Concat_StrStr` (`KismetTextLibrary.Conv_TextToString` (`|FormatText` "Time: ")) (`KismetStringLibrary.Conv_IntToString` _currenttime_hour) ":" (`KismetStringLibrary.Conv_IntToString` _currenttime_minute)))))))

(event `OpenInteract`
  (bind _returnvalue (`GameplayStatics.GetPlayerController` 0))
  (bind _interactmenu (`self.InteractMenu`))
  (`Widget.SetVisibility` _interactmenu "Visible")
  (`WidgetBlueprintLibrary.SetInputMode_UIOnlyEx` _returnvalue _interactmenu "LockAlways" true)
  (set `PlayerController.bShowMouseCursor` true _returnvalue))

(event `Hit`
  (bind _interactednpc (`self.InteractedNPC`))
  (set `self.Interacting` true)
  (if (`KismetSystemLibrary.IsValid` _interactednpc)
    (`Widget.SetVisibility` (`self.InteractMenu`) "Collapsed")
    (`/Game/Villagers/SkeletonVillagers/BaseVillager_BP.Hit` _interactednpc)
    (`Widget.SetVisibility` (`self.Textbox`) "Visible")
    (`self.AllowInput`)))

(event `CleanUI`
  (`Widget.SetVisibility` (`self.Textbox`) "Collapsed"))

(event `AllowInput`
  (bind _returnvalue (`GameplayStatics.GetPlayerController` 0))
  (`WidgetBlueprintLibrary.SetInputMode_GameOnly` _returnvalue)
  (set `PlayerController.bShowMouseCursor` false _returnvalue))

(event `Gift`
  (set `self.Interacting` true)
  (if (`KismetSystemLibrary.IsValid` (`self.InteractedNPC`))
    (`Widget.SetVisibility` (`self.InteractMenu`) "Collapsed")
    (`Widget.SetVisibility` (`self.GiftName`) "Visible")))

(event `Talk`
  (set `self.Interacting` true)
  (if (`KismetSystemLibrary.IsValid` (`self.InteractedNPC`))
    (`Widget.SetVisibility` (`self.InteractMenu`) "Collapsed")
    (`Widget.SetVisibility` (`self.DialogMenu`) "Visible")))

(event `GiftReceipt`
  (params (Name :type String))
  (`Widget.SetVisibility` (`self.GiftName`) "Collapsed")
  (`/Game/Villagers/SkeletonVillagers/BaseVillager_BP.Gift` (`self.InteractedNPC`) Name)
  (`Widget.SetVisibility` (`self.Textbox`) "Visible")
  (`self.AllowInput`))

(event `TalkAboutMood`
  (`Widget.SetVisibility` (`self.DialogMenu`) "Collapsed")
  (`/Game/Villagers/SkeletonVillagers/BaseVillager_BP.Talk` (`self.InteractedNPC`) "Mood")
  (`Widget.SetVisibility` (`self.Textbox`) "Visible" :!label _label)
  (`self.AllowInput`))

(event `TalkAboutEnergy`
  (`Widget.SetVisibility` (`self.DialogMenu`) "Collapsed")
  (`/Game/Villagers/SkeletonVillagers/BaseVillager_BP.Talk` (`self.InteractedNPC`) "Energy")
  (goto _label))

(event `TalkAboutRelationship`
  (`Widget.SetVisibility` (`self.DialogMenu`) "Collapsed")
  (`/Game/Villagers/SkeletonVillagers/BaseVillager_BP.Talk` (`self.InteractedNPC`) "Relationship")
  (goto _label))

(event `Talk about anything`
  (`Widget.SetVisibility` (`self.DialogMenu`) "Collapsed")
  (`/Game/Villagers/SkeletonVillagers/BaseVillager_BP.Talk` (`self.InteractedNPC`) "Anything")
  (goto _label))

(event `TalkAboutGeneric`
  (`Widget.SetVisibility` (`self.DialogMenu`) "Collapsed")
  (`/Game/Villagers/SkeletonVillagers/BaseVillager_BP.Talk` (`self.InteractedNPC`) "Generic")
  (goto _label))

(event `TalkAboutJob`
  (`Widget.SetVisibility` (`self.DialogMenu`) "Collapsed")
  (`/Game/Villagers/SkeletonVillagers/BaseVillager_BP.Talk` (`self.InteractedNPC`) "Job")
  (goto _label))

(event `Talk About Coworkers`
  (`Widget.SetVisibility` (`self.DialogMenu`) "Collapsed")
  (`/Game/Villagers/SkeletonVillagers/BaseVillager_BP.Talk` (`self.InteractedNPC`) "Coworker")
  (goto _label))

(fn `UserConstructionScript`)